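; BP_PlayerCidara is the player character Blueprint for Cidara, extending a parent class whose tick and construction it calls.
; On its first tick, a DoOnce caches the BP_GI_Cidara game instance and adds the IMC_PlayerCidara Enhanced Input mapping context to the owning player controller's subsystem.
; This one-time setup runs in Tick rather than BeginPlay, before the parent tick is called.
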(event EventTick
  (params (DeltaSeconds :type Float%20%28single-precision%29))
  (Utilities|FlowControl|Sequence
    (:then_0
      (Utilities|FlowControl|DoOnce false
        (:Completed
          (Utilities|FlowControl|Sequence
            (:then_0
              (bind _asbp_gi_cidara (Utilities|Casting|CastToBP_GI_Cidara (Game|GetGameInstance)))
              (Variables|Default|SetGameInstanceRef _asbp_gi_cidara))
            (:then_1
              (bind _asplayer_controller (Utilities|Casting|CastToPlayerController (Pawn|GetController)))
              (Utilities|IsValid (PlayerController|LocalPlayerSubsystems|GetEnhancedInputLocalPlayerSubsystem _asplayer_controller)
                (:Is%20Valid
                  (Input|AddMappingContext (PlayerController|LocalPlayerSubsystems|GetEnhancedInputLocalPlayerSubsystem _asplayer_controller) "/Game/Game/Input/IMC_PlayerCidara.IMC_PlayerCidara" 0 "(bIgnoreAllPressedKeysUntilRelease=True,bForceImmediately=False,bNotifyUserSettings=False)"))))))))
    (:then_1
      (|CallParentFunction 0.0))))

(fn ConstructionScript
  (|CallParentFunction))