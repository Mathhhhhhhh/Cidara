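; BP_CamSpectre is a Spectre camera-manager Blueprint that handles input for switching characters and climbing.
; Pressing E activates Cidara's CharacterMovement component and has the current controller possess Cidara.
; Pressing R toggles climbing by checking the Spectre's IsClimbing flag, then calling SpectreClimb or StopClimbing on it.
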(event Input|KeyboardEvents|E
  (params (Key :type Key%20Structure :default "None"))
  ;[1 1 1 0.5] possess cidara
  (:Pressed
    (Components|Activation|Activate (Variables|/Script/Engine.Character|GetCharacterMovement (Variables|Default|GetCidara)) false)
    (Pawn|Possess (Pawn|GetController) (Variables|Default|GetCidara))))

(event Input|KeyboardEvents|R
  (params (Key :type Key%20Structure :default "None"))
  (bind _spectre (Variables|Default|GetSpectre))
  ;[1 1 1] Start Climb
  (:Pressed
    (if (not (Variables|/Game/Game/Blueprints/Characters/Spectre/BP_Spectre.BP_Spectre_C|GetisClimbing? _spectre))
      (Default|SpectreClimb _spectre)
      (else
        (Default|StopClimbing _spectre)))))

(fn ConstructionScript)